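; BP_Dalek is a Dalek AI pawn that chases the player character once it spots a pawn.
; It caches the player on BeginPlay, and its PawnSensing see event sets a seen flag and calls FollowPlayer, which runs AI MoveTo toward that player.
; Reaching the player only clears CanAttack, with no attack action, and the seen flag is never reset here.
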(event `self.ReceiveBeginPlay`
  (bind _asbp_player (cast `/Game/Blueprint/Player/BP_Player` (`GameplayStatics.GetPlayerCharacter` 0)))
  (set `self.As BP_Player` _asbp_player))

(event `self.PawnSensing.OnSeePawn`
  (params (Pawn :type "Pawn Object Reference"))
  (set `self.isSeeingPlayer?` true)
  (`self.FollowPlayer`))

(event `FollowPlayer`
  (set `self.CanAttack?` true)
  (if (`self.isSeeingPlayer?`)
    (`|AIMoveTo` self (0.0 0.0 0.0) (`self.As BP_Player`) 100.0
      (:`OnSuccess`
        (if (`self.CanAttack?`)
          (set `self.CanAttack?` false))))))

(fn `UserConstructionScript`)