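; Dalek enemy that chases the player on sight and triggers the game over display when it catches them.
; PawnSensing calls FollowPlayer, which uses AI MoveTo toward the cached BP_Player.
; On arrival, a call counter ensures the Doctor Who sound and game over visibility fire only once.
; StopDalek and ReactivateDalek toggle a cinematic flag that blocks new chase requests without cancelling an active move.
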(event `self.ReceiveBeginPlay`
  (bind _asbp_player (cast `/Game/Blueprint/Player/BP_Player` (`GameplayStatics.GetPlayerCharacter` 0)))
  (set `self.As BP_Player` _asbp_player))

(event `self.PawnSensing.OnSeePawn`
  (params (Pawn :type "Pawn Object Reference"))
  (set `self.isSeeingPlayer?` true)
  (`self.FollowPlayer`))

(event `FollowPlayer`
  (bind _nb_call (`self.nb_call`))
  (if (not (`self.IsInCinematique`))
    (set `self.CanAttack?` true)
    (if (`self.isSeeingPlayer?`)
      (`|AIMoveTo` self (0.0 0.0 0.0) (`self.As BP_Player`) 200.0
        (:`OnSuccess`
          (if (`self.CanAttack?`)
            (set `self.CanAttack?` false)
            (if (== _nb_call 0)
              (`GameplayStatics.PlaySound2D` "/Game/Music/Dalek/Doctor_Who.Doctor_Who" 1.0 1.0 0.0 null null)
              (`/Engine/EditorBlueprintResources/StandardMacros.IncrementInt` _nb_call
                (:`  `
                  (`/Game/Blueprint/Player/BP_Player.Set Visibility for GameOver` (`self.As BP_Player`) "Visible"))))))))))

(event `Stop Dalek`
  (set `self.IsInCinematique` true))

(event `Reactivate Dalek`
  (set `self.IsInCinematique` false))

(fn `UserConstructionScript`)