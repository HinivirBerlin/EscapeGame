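; BP_Cristal_Orb is an interactable crystal ball that opens a door once its orb count reaches 13.
; Tick reveals the initially hidden NSBasic9 effect when NbOrb reaches that threshold.
; Interact then plays a sound, opens the referenced Door, hides the effect and resets the count.
; Box overlaps toggle a green highlight overlay material on the ball; this file never increments NbOrb.
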(event `self.ReceiveBeginPlay`
  (`SceneComponent.SetVisibility` (`self.NS_Basic_9`) false false))

(event `self.ReceiveTick`
  (params (DeltaSeconds :type "Float (single-precision)"))
  (if (not (< (`self.Nb_Orb`) 13))
    (`SceneComponent.SetVisibility` (`self.NS_Basic_9`) true false)))

(event `self.Box.OnComponentBeginOverlap`
  (params (OverlappedComponent :type "PrimitiveComponent Object Reference") (OtherActor :type "Actor Object Reference") (OtherComp :type "PrimitiveComponent Object Reference") (OtherBodyIndex :type Integer) (bFromSweep :type Boolean) (SweepResult :type "HitResult Structure (by ref)"))
  (`MeshComponent.SetOverlayMaterial` (`self.crystal_ball`) "/Game/Material/MI_HighlightGreen.MI_HighlightGreen"))

(event `self.Box.OnComponentEndOverlap`
  (params (OverlappedComponent :type "PrimitiveComponent Object Reference") (OtherActor :type "Actor Object Reference") (OtherComp :type "PrimitiveComponent Object Reference") (OtherBodyIndex :type Integer))
  (`MeshComponent.SetOverlayMaterial` (`self.crystal_ball`) null))

(event `self.Interact`
  (params (Interactor :type "Character Object Reference"))
  (if (not (< (`self.Nb_Orb`) 13))
    (`GameplayStatics.PlaySound2D` "/Engine/VREditor/Sounds/UI/Dockable_Window_Close.Dockable_Window_Close" 1.0 1.0 0.0 null null)
    (`/Game/Blueprints/Door_Level/BP_Parent_Door.Open_Door` (`self.Door`))
    (`SceneComponent.SetVisibility` (`self.NS_Basic_9`) false false)
    (set `self.Nb_Orb` 0)))

(fn `UserConstructionScript`)