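; BP_Earth_Invisible is a solar system Earth that stays hidden until three planets have been returned, apparently as a puzzle that unlocks a door.
; It hides its EarthAndClouds component on BeginPlay and increments a counter on each Planetreturn event.
; When TurnVisible is called with the counter at exactly three, it shows EarthAndClouds and calls OpenDoor on the referenced Door.
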(event `Planet return`
  (`/Engine/EditorBlueprintResources/StandardMacros.IncrementInt` (`self.Number_Planet`)))

(event `self.ReceiveBeginPlay`
  (`SceneComponent.SetVisibility` (`self.earth_and_clouds`) false false))

(event `Turn Visible`
  (if (== (`self.Number_Planet`) 3)
    (`SceneComponent.SetVisibility` (`self.earth_and_clouds`) true false)
    (`/Game/Blueprints/Door_Level/BP_Parent_Door.Open_Door` (`self.Door`))))

(fn `UserConstructionScript`)