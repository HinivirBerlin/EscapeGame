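; Level 6 chase trigger that starts a Dalek sequence when interacted with.
; On Interact, it opens its referenced door, calls for a cinematic and tells the Dalek reference to spawn a Dalek.
; A DalekNumber counter gates the sequence to a single run, assuming it starts at zero, and is printed as debug output.
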(event `/Game/Blueprint/BPI_Interact.Interact`
  (params (Interactor :type "Character Object Reference"))
  (bind _dalek_number (`self.Dalek_number`))
  (if (< _dalek_number 1)
    (bind _result (`/Engine/EditorBlueprintResources/StandardMacros.IncrementInt` _dalek_number)
      (:`  `
        (`KismetSystemLibrary.PrintString` (`KismetStringLibrary.Conv_IntToString` _result))
        (`/Game/Blueprints/Door_Level/BP_Parent_Door.Open_Door` (`self.Door`))
        (`self.Call_cinematic`)
        (`/Game/Blueprints/Dalek/BP_Spawner.SpawnDalek` (`self.Dalek`))))))

(fn `UserConstructionScript`)