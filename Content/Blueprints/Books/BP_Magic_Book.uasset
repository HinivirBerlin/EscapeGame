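; BP_Magic_Book is an interactable magic book that plays a low witch laugh when used.
; Interact calls Laugh, which plays the 2D sound and uses an Isplaying flag with a seven-second delay to block overlapping replays.
; A Box trigger applies a green highlight overlay material to the book mesh on any overlap and clears it when the overlap ends.
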(event `Laugh`
  (if (not (`self.isplaying`))
    (set `self.isplaying` true)
    (`GameplayStatics.PlaySound2D` "/Game/Music/Witch_Laugh_Low.Witch_Laugh_Low" 1.0 1.0 0.0 null null)
    (`KismetSystemLibrary.Delay` 7.0)
    (set `self.isplaying` false)))

(event `/Game/Blueprint/BPI_Interact.Interact`
  (params (Interactor :type "Character Object Reference"))
  (`self.Laugh`))

(event `self.Box.OnComponentBeginOverlap`
  (params (OverlappedComponent :type "PrimitiveComponent Object Reference") (OtherActor :type "Actor Object Reference") (OtherComp :type "PrimitiveComponent Object Reference") (OtherBodyIndex :type Integer) (bFromSweep :type Boolean) (SweepResult :type "HitResult Structure (by ref)"))
  (`MeshComponent.SetOverlayMaterial` (`self.free_the_magic_book_game_ready_asset`) "/Game/Material/MI_HighlightGreen.MI_HighlightGreen"))

(event `self.Box.OnComponentEndOverlap`
  (params (OverlappedComponent :type "PrimitiveComponent Object Reference") (OtherActor :type "Actor Object Reference") (OtherComp :type "PrimitiveComponent Object Reference") (OtherBodyIndex :type Integer))
  (`MeshComponent.SetOverlayMaterial` (`self.free_the_magic_book_game_ready_asset`) null))

(fn `UserConstructionScript`)