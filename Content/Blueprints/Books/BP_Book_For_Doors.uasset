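; BP_Book_For_Doors is an interactable book actor that serves as a trigger for opening a door.
; Interact calls OpenDoor, while the Open_Door event plays a ping sound, opens the referenced Door and destroys the book.
; Box overlap events apply a green highlight overlay material to the book mesh on entry and clear it on exit, with no filter on the overlapping actor.
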(event `Open_Door`
  (`GameplayStatics.PlaySound2D` "/Engine/EngineSounds/1kSineTonePing.1kSineTonePing" 1.0 1.0 0.0 null null)
  (`/Game/Blueprints/Door_Level/BP_Parent_Door.Open_Door` (`self.Door`))
  (`self.K2_DestroyActor`))

(event `/Game/Blueprint/BPI_Interact.Interact`
  (params (Interactor :type "Character Object Reference"))
  (`self.Open_Door`))

(event `self.Box.OnComponentBeginOverlap`
  (params (OverlappedComponent :type "PrimitiveComponent Object Reference") (OtherActor :type "Actor Object Reference") (OtherComp :type "PrimitiveComponent Object Reference") (OtherBodyIndex :type Integer) (bFromSweep :type Boolean) (SweepResult :type "HitResult Structure (by ref)"))
  (`MeshComponent.SetOverlayMaterial` (`self.Book_LOD0`) "/Game/Material/MI_HighlightGreen.MI_HighlightGreen"))

(event `self.Box.OnComponentEndOverlap`
  (params (OverlappedComponent :type "PrimitiveComponent Object Reference") (OtherActor :type "Actor Object Reference") (OtherComp :type "PrimitiveComponent Object Reference") (OtherBodyIndex :type Integer))
  (`MeshComponent.SetOverlayMaterial` (`self.Book_LOD0`) null))

(fn `UserConstructionScript`)