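; Door actor in the Lasers game that opens and closes through its BPAC_External component's activate and deactivate events.
; Activation plays a 2D sound, then hides the Cube and disables its collision.
; Deactivation shows the Cube and restores its collision without a sound.
; BeginPlay caches the Cube's world location, but the nodes that would move the door are disconnected, so it never moves.
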(event `self.ReceiveBeginPlay`
  (set `self.NewVar` (`SceneComponent.K2_GetComponentLocation` (`self.Cube`))))

(event `self.BPAC_External.ExternalActivate`
  (params (ApplyConditions :type Boolean))
  (bind _cube (`self.Cube`))
  (`GameplayStatics.PlaySound2D` "/Engine/VREditor/Sounds/UI/Teleport_Committed.Teleport_Committed" 1.0 1.0 0.0 null null)
  (`PrimitiveComponent.SetCollisionEnabled` _cube "NoCollision")
  (`SceneComponent.SetHiddenInGame` _cube true false))

(event `self.BPAC_External.ExternalDeactivate`
  (params (ApplyConditions :type Boolean))
  (bind _cube (`self.Cube`))
  (`PrimitiveComponent.SetCollisionEnabled` _cube "QueryAndPhysics")
  (`SceneComponent.SetHiddenInGame` _cube false false))

(fn `UserConstructionScript`)