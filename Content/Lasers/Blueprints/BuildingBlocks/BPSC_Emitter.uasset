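; Scene component that emits a laser in the laser system, driven by hit events and the BPAC_Handler found on its owner.
; On activation it spawns and attaches a BPA_Laser, passing color, range and previous lasers, and ignoring the owner.
; Spawning depends on the handler's activation check and optional color matching against merged or individual incoming lasers.
; Inverted systems swap hit start and stop behavior, while forced events allow direct switching.
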(event `self.ReceiveBeginPlay`
  (bind _returnvalue (`Actor.GetComponentByClass` (`self.GetOwner`) "/Game/Lasers/Blueprints/BuildingBlocks/BPAC_Handler.BPAC_Handler_C"))
  (`/Engine/EditorBlueprintResources/StandardMacros.IsValid` _returnvalue
    (:`Is Valid`
      (set `self.Owning Handler` _returnvalue))))

(event `/Game/Lasers/Blueprints/BuildingBlocks/BPI_Lasers.Laser Start Hitting`
  (params (Input :type "/Game/Lasers/Blueprints/BuildingBlocks/BPA_Laser Object Reference") (`Hit Info` :type "HitResult Structure"))
  (if (`self.IsSystemInverted`)
    (if (`self.CanSpawnLaser`)
      (`self.Deactivate Laser`))
    (else
      (`self.Set Laser Color` :!label _label)
      (if (`self.CanSpawnLaser`)
        (`self.Attached Laser` :!label _label_2
          (:`then`)
          (:`else`
            (`self.Activate Laser`)))))))

(event `/Game/Lasers/Blueprints/BuildingBlocks/BPI_Lasers.ForceActivation`
  (params (ApplyConditions :type Boolean))
  (if ApplyConditions
    (goto _label)
    (else
      (`self.Set Laser Color`)
      (goto _label_2))))

(event `/Game/Lasers/Blueprints/BuildingBlocks/BPI_Lasers.Laser Stop Hitting`
  (params (Input :type "/Game/Lasers/Blueprints/BuildingBlocks/BPA_Laser Object Reference"))
  (if (`self.IsSystemInverted`)
    (if (`self.CanSpawnLaser`)
      (`self.Attached Laser`
        (:`then`)
        (:`else`
          (`self.Activate Laser`))))
    (elif (not (`self.CanSpawnLaser`))
      (`self.Deactivate Laser` :!label _label_3))))

(event `/Game/Lasers/Blueprints/BuildingBlocks/BPI_Lasers.ForceDeactivation`
  (params (ApplyConditions :type Boolean))
  (goto _label_3))

(event `/Game/Lasers/Blueprints/BuildingBlocks/BPI_Lasers.Intermediate Change`
  (params (Modified :type "/Game/Lasers/Blueprints/BuildingBlocks/BPA_Laser Object Reference"))
  (if (not (`self.IsSystemInverted`))
    (`self.Set Laser Color`)
    (if (`self.CanSpawnLaser`)
      (`self.Attached Laser`
        (:`then`)
        (:`else`
          (`self.Activate Laser`)))
      (else
        (`self.Deactivate Laser`)))))

(fn `Activate Laser`
  (bind _returnvalue (`|SpawnActorFromClass` "/Game/Lasers/Blueprints/BuildingBlocks/BPA_Laser.BPA_Laser_C" (`self.K2_GetComponentToWorld`) "Undefined" "MultiplyWithRoot" null (`self.Current Color`) (`self.MaxRange`) (`self.Get FIltered Lasers`) (`self.Owning Handler`) (`|MakeArray` (`self.GetOwner`)) null))
  (bind _output_get (set `self.Attached Laser` _returnvalue))
  (`Actor.K2_AttachToComponent` _output_get self "None" "KeepWorld" "KeepWorld" "KeepWorld" false))

(fn `CanSpawnLaser`
  (returns (OutputPin :type Boolean))
  (if (`/Game/Lasers/Blueprints/BuildingBlocks/BPAC_Handler.IsAdjustingColor` (`self.Owning Handler`))
    (if (`/Game/Lasers/Blueprints/BuildingBlocks/BPAC_Handler.CanMergeColor` (`self.Owning Handler`))
      (return (and (`/Game/Lasers/Blueprints/BuildingBlocks/BPAC_Handler.DoesContainColor` (`self.Owning Handler`) (`/Game/Lasers/Blueprints/BuildingBlocks/BPAC_Handler.GetMergedColor` (`self.Owning Handler`)) (`self.Override Color`)) (`/Game/Lasers/Blueprints/BuildingBlocks/BPAC_Handler.CanActivate` (`self.Owning Handler`))))
      (else
        (for _array_element (`self.Get FIltered Lasers`)
          (if (and (`/Game/Lasers/Blueprints/BuildingBlocks/BPAC_Handler.DoesContainColor` (`self.Owning Handler`) (`/Game/Lasers/Blueprints/BuildingBlocks/BPA_Laser.ColorOverride` _array_element) (`self.Override Color`)) (`/Game/Lasers/Blueprints/BuildingBlocks/BPAC_Handler.CanActivate` (`self.Owning Handler`)))
            (return true)))
        (return false)))
    (else
      (return (`/Game/Lasers/Blueprints/BuildingBlocks/BPAC_Handler.CanActivate` (`self.Owning Handler`))))))

(fn `Deactivate Laser`
  (bind _attached_laser (`self.Attached Laser`)
    (:`then`
      (`/Game/Lasers/Blueprints/BuildingBlocks/BPA_Laser.Laser Stop Hitting` _attached_laser null))
    (:`else`)))

(fn `DestroySelf`
  (`self.K2_DestroyComponent`))

(fn `Set Laser Color`
  (locals (`L-TempColor` :type "LinearColor Structure"))
  (`|ExecutionSequence`
    (:`then_0`
      (if (`self.Use Override`)
        (set `local.L-TempColor` (`self.Override Color`))
        (elif true
          (set `local.L-TempColor` (`self.Current Color`))
          (else
            (set `local.L-TempColor` (`/Game/Lasers/Blueprints/BuildingBlocks/BPAC_Handler.GetVisibleColor` (`self.Owning Handler`)))))))
    (:`then_1`
      (if (!= (`self.Current Color`) (`local.L-TempColor`))
        (set `self.Current Color` (`local.L-TempColor`))
        (bind _attached_laser (`self.Attached Laser`)
          (:`then`
            (`/Game/Lasers/Blueprints/BuildingBlocks/BPA_Laser.ChangeLaserColor` _attached_laser (`self.Current Color`)))
          (:`else`))))))