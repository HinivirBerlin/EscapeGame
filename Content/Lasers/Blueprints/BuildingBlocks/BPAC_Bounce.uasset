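; Actor component that makes its owner bounce lasers, acting as a reflective surface in the laser building-block system.
; When a new laser starts hitting, it spawns and activates a BPSC_Emitter on the owner at the mirrored hit transform, stored in a map keyed by incoming laser.
; Hit updates move that emitter to follow the reflection.
; When the hit stops, it shuts down, destroys and unmaps the emitter.
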(event `self.ReceiveBeginPlay`
  (bind _returnvalue (`Actor.GetComponentByClass` (`self.GetOwner`) "/Game/Lasers/Blueprints/BuildingBlocks/BPAC_Handler.BPAC_Handler_C"))
  (`/Engine/EditorBlueprintResources/StandardMacros.IsValid` _returnvalue
    (:`Is Valid`
      (set `self.Owning Handler` _returnvalue))))

(event `/Game/Lasers/Blueprints/BuildingBlocks/BPI_Lasers.Laser Start Hitting`
  (params (Input :type "/Game/Lasers/Blueprints/BuildingBlocks/BPA_Laser Object Reference") (`Hit Info` :type "HitResult Structure"))
  (`/Engine/EditorBlueprintResources/StandardMacros.IsValid` Input
    (:`Is Valid`
      (if (not (`BlueprintMapLibrary.Map_Contains` (`self.EmiterBounceMap`) Input))
        (`self.Spawn Laser` Input `Hit Info`)))))

(event `/Game/Lasers/Blueprints/BuildingBlocks/BPI_Lasers.Laser Stop Hitting`
  (params (Input :type "/Game/Lasers/Blueprints/BuildingBlocks/BPA_Laser Object Reference"))
  (`self.Remove Laser` Input))

(event `/Game/Lasers/Blueprints/BuildingBlocks/BPI_Lasers.Laser Update Hitting`
  (params (Input :type "/Game/Lasers/Blueprints/BuildingBlocks/BPA_Laser Object Reference") (`Hit Info` :type "HitResult Structure"))
  (bind (_location _rotation) (`self.Mirror Location Rotation` `Hit Info`))
  (bind (_value _returnvalue) (`BlueprintMapLibrary.Map_Find` (`self.EmiterBounceMap`) Input))
  (if _returnvalue
    (`SceneComponent.K2_SetWorldLocationAndRotation` _value _location _rotation false false)))

(fn `Remove Laser`
  (params (InputPin :type "/Game/Lasers/Blueprints/BuildingBlocks/BPA_Laser Object Reference"))
  (locals (`L-Remove` :type "/Game/Lasers/Blueprints/BuildingBlocks/BPSC_Emitter Object Reference"))
  (bind (_value _returnvalue) (`BlueprintMapLibrary.Map_Find` (`self.EmiterBounceMap`) (`local.InputPin`)))
  (if _returnvalue
    (bind _output_get (set `local.L-Remove` _value))
    (`/Game/Lasers/Blueprints/BuildingBlocks/BPSC_Emitter.Laser Stop Hitting` _output_get null)
    (`self.K2_DestroyComponent` (`local.L-Remove`))
    (`BlueprintMapLibrary.Map_Remove` (`self.EmiterBounceMap`) (`local.InputPin`))))

(fn `Spawn Laser`
  (params (`Laser In` :type "/Game/Lasers/Blueprints/BuildingBlocks/BPA_Laser Object Reference") (`Hit Info` :type "HitResult Structure"))
  (bind _returnvalue (`Actor.GetTransform` (`self.GetOwner`)))
  (bind (_location _rotation) (`self.Mirror Location Rotation` (`local.Hit Info`)))
  (bind _returnvalue_2 (`|AddComponentByClass` (`self.GetOwner`) "/Game/Lasers/Blueprints/BuildingBlocks/BPSC_Emitter.BPSC_Emitter_C" false (`KismetMathLibrary.MakeTransform` (`KismetMathLibrary.InverseTransformLocation` _returnvalue _location) (`KismetMathLibrary.InverseTransformRotation` _returnvalue _rotation))))
  (`BlueprintMapLibrary.Map_Add` (`self.EmiterBounceMap`) (`local.Laser In`) _returnvalue_2)
  (`/Game/Lasers/Blueprints/BuildingBlocks/BPSC_Emitter.Activate Laser` _returnvalue_2))