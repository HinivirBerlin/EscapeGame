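; BPA_Laser is a laser beam actor that detects and notifies objects carrying a BPAC_Handler component.
; Each Tick it multi-traces forward, scales the mesh to the blocking hit or full range, and diffs handler sets to send start, update and stop messages.
; A recursive check through PreviousLasers skips handlers already upstream, preventing loops in laser chains.
; Color changes update a dynamic material and notify previously hit handlers.
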(event `self.ReceiveBeginPlay`
  (bind _returnvalue (`KismetMaterialLibrary.CreateDynamicMaterialInstance` "/Game/Lasers/Materiels/MI_Laser.MI_Laser"))
  (set `self.Materil Instance` _returnvalue)
  (`PrimitiveComponent.SetMaterial` (`self.StaticMesh`) 0 (`self.Materil Instance`))
  (`self.ChangeLaserColor` (`self.ColorOverride`)))

(event `self.ReceiveTick`
  (params (DeltaSeconds :type "Float (single-precision)"))
  (bind _returnvalue (`self.K2_GetActorLocation`))
  (bind (_outhits _returnvalue_2) (`KismetSystemLibrary.LineTraceMulti` _returnvalue (+ _returnvalue (* (`self.GetActorForwardVector`) (`self.Range`))) "TraceTypeQuery3" false (`self.Actors To Ignore`)))
  (if _returnvalue_2
    (for _array_element _outhits
      (`|ExecutionSequence`
        (:`then_0`
          (bind (_bblockinghit _binitialoverlap _time _distance) (`GameplayStatics.BreakHitResult` _array_element))
          (if _bblockinghit
            (`self.Update Lenght` _distance)))
        (:`then_1`
          (`self.Handle Hit Actor` _array_element))))
    (else
      (`self.Update Lenght` (`self.Range`))))
  (bind _result (`BlueprintSetLibrary.Set_Difference` (`self.Previously Hit Handlers`) (`self.Current Hit Handler`)))
  (bind _result_2 (`BlueprintSetLibrary.Set_ToArray` _result))
  (for _array_element_2 _result_2
    (message `/Game/Lasers/Blueprints/BuildingBlocks/BPI_Lasers.Laser Stop Hitting` _array_element_2 self)
    (`BlueprintMapLibrary.Map_Remove` (`self.Hitting Handlers`) _array_element_2))
  (set `self.Previously Hit Handlers` (`self.Current Hit Handler`))
  (`BlueprintSetLibrary.Set_Clear` (`self.Current Hit Handler`)))

(event `/Game/Lasers/Blueprints/BuildingBlocks/BPI_Lasers.Laser Stop Hitting`
  (params (Input :type "/Game/Lasers/Blueprints/BuildingBlocks/BPA_Laser Object Reference"))
  (`|ExecutionSequence`
    (:`then_0`
      (bind _result (`BlueprintSetLibrary.Set_ToArray` (`self.Previously Hit Handlers`)))
      (for _array_element _result
        (message `/Game/Lasers/Blueprints/BuildingBlocks/BPI_Lasers.Laser Stop Hitting` _array_element self)))
    (:`then_1`
      (`self.K2_DestroyActor`))))

(fn `ChangeLaserColor`
  (params (Value :type "LinearColor Structure"))
  (set `self.ColorOverride` Value)
  (`MaterialInstanceDynamic.SetVectorParameterValue` (`self.Materil Instance`) "Color" (`self.ColorOverride`))
  (bind _result (`BlueprintSetLibrary.Set_ToArray` (`self.Previously Hit Handlers`)))
  (for _array_element _result
    (`/Game/Lasers/Blueprints/BuildingBlocks/BPAC_Handler.Intermediate Change` _array_element self)))

(fn `GetHitByHandler`
  (params (Key :type "/Game/Lasers/Blueprints/BuildingBlocks/BPAC_Handler Object Reference (by ref)"))
  (returns (Value :type "HitResult Structure") (ReturnValue :type Boolean))
  (bind (_value _returnvalue) (`BlueprintMapLibrary.Map_Find` (`self.Hitting Handlers`) (`local.Key`)))
  (return _value _returnvalue))

(fn `Handle Hit Actor`
  (params (InputPin :type "HitResult Structure"))
  (locals (`L-Handler` :type "/Game/Lasers/Blueprints/BuildingBlocks/BPAC_Handler Object Reference"))
  (bind _returnvalue (`self.GetComponentByClass` (`.HitActor` (`GameplayStatics.BreakHitResult` InputPin)) "/Game/Lasers/Blueprints/BuildingBlocks/BPAC_Handler.BPAC_Handler_C"))
  (`/Engine/EditorBlueprintResources/StandardMacros.IsValid` _returnvalue
    (:`Is Valid`
      (set `local.L-Handler` _returnvalue)
      (if (`self.Is Not On Path` (`local.L-Handler`))
        (`BlueprintMapLibrary.Map_Add` (`self.Hitting Handlers`) (`local.L-Handler`) (`local.InputPin`))
        (if (`BlueprintSetLibrary.Set_Contains` (`self.Previously Hit Handlers`) (`local.L-Handler`))
          (`/Game/Lasers/Blueprints/BuildingBlocks/BPAC_Handler.Laser Update Hitting` (`local.L-Handler`) self (`local.InputPin`))
          (else
            (message `/Game/Lasers/Blueprints/BuildingBlocks/BPI_Lasers.Laser Start Hitting` (`local.L-Handler`) self (`local.InputPin`))))
        (`BlueprintSetLibrary.Set_Add` (`self.Current Hit Handler`) (`local.L-Handler`))))))

(fn `Is Not On Path`
  (params (InputPin :type "ActorComponent Object Reference"))
  (returns (OutputPin :type Boolean))
  (locals (`L-CurrentLaser` :type "/Game/Lasers/Blueprints/BuildingBlocks/BPA_Laser Object Reference"))
  (if (`KismetArrayLibrary.Array_IsNotEmpty` (`self.PreviousLasers`))
    (for _array_element (`self.PreviousLasers`)
      (bind _output_get (set `local.L-CurrentLaser` _array_element))
      (if (== (`/Game/Lasers/Blueprints/BuildingBlocks/BPA_Laser.Owning Handler` _output_get) (`local.InputPin`))
        (return false)
        (elif (not (`self.Is Not On Path` (`local.L-CurrentLaser`) (`local.InputPin`)))
          (return false))))
    (return true)
    (else
      (return true))))

(fn `Update Lenght`
  (params (InputPin :type "Float (single-precision)"))
  (if (not (`KismetMathLibrary.NearlyEqual_FloatFloat` InputPin (`self.PreviousLenght`) 2.0))
    (bind _output_get (set `self.PreviousLenght` (`local.InputPin`)))
    (`SceneComponent.SetWorldScale3D` (`self.StaticMesh`) (`KismetMathLibrary.MakeVector` 0.1 0.1 (/ _output_get 100.0)))))

(fn `UserConstructionScript`)