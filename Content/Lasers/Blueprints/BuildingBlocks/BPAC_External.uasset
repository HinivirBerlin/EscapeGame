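; Laser building-block component that links its owner to BPAC_Handler components on target actors, relaying activation for objects like doors.
; By default it tracks handler states in a map and rebroadcasts their activate, deactivate and update events, gating activation on AllActorsActive, whose loop is left unwired.
; InvertControl reverses the link: it registers itself with each handler, binds its own External dispatchers and fires them without that check.
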(event `self.ReceiveBeginPlay`
  (if (`KismetArrayLibrary.Array_IsNotEmpty` (`self.TargetActors`))
    (`self.LinkDelegates`)))

(event `LinkDelegates`
  (if (`self.InvertControl`)
    (for _array_element (`self.TargetActors`)
      (bind _returnvalue (`Actor.GetComponentByClass` _array_element "/Game/Lasers/Blueprints/BuildingBlocks/BPAC_Handler.BPAC_Handler_C"))
      (`/Engine/EditorBlueprintResources/StandardMacros.IsValid` _returnvalue
        (:`Is Valid`
          (`KismetArrayLibrary.Array_AddUnique` (`/Game/Lasers/Blueprints/BuildingBlocks/BPAC_Handler.LinkedExternalComps` _returnvalue) self)
          (add `self.ExternalActivate` (`|CreateDelegate` _returnvalue :!event `ForceActivation`))
          (add `self.ExternalDeactivate` (`|CreateDelegate` _returnvalue :!event `ForceDeactivation`)))))
    (else
      (for _array_element_2 (`self.TargetActors`)
        (bind _returnvalue_2 (`Actor.GetComponentByClass` _array_element_2 "/Game/Lasers/Blueprints/BuildingBlocks/BPAC_Handler.BPAC_Handler_C"))
        (`/Engine/EditorBlueprintResources/StandardMacros.IsValid` _returnvalue_2
          (:`Is Valid`
            (`BlueprintMapLibrary.Map_Add` (`self.NecessaryActors`) _returnvalue_2 (`/Game/Lasers/Blueprints/BuildingBlocks/BPAC_Handler.Invert System` _returnvalue_2))
            (add `/Game/Lasers/Blueprints/BuildingBlocks/BPAC_Handler.ActivateHandler` _returnvalue_2 (`|CreateDelegate` :!event `Activate This`))
            (add `/Game/Lasers/Blueprints/BuildingBlocks/BPAC_Handler.DeactivateHandler` _returnvalue_2 (`|CreateDelegate` :!event `Deactivate This`))
            (add `/Game/Lasers/Blueprints/BuildingBlocks/BPAC_Handler.UpdateHandler` _returnvalue_2 (`|CreateDelegate` :!event `Update This`))))))))

(fn `Activate This`
  (params (Instigator :type "/Game/Lasers/Blueprints/BuildingBlocks/BPAC_Handler Object Reference"))
  (if (`self.InvertControl`)
    (set `self.IsCompActivated` true)
    (`self.ExternalActivate` (`self.ApplyConditions`))
    (else
      ;[1 1 1] Used in cases like Doors
      (`|ExecutionSequence`
        (:`then_0`
          (`BlueprintMapLibrary.Map_Add` (`self.NecessaryActors`) (`local.Instigator`) true))
        (:`then_1`
          (if (`self.AllActorsActive`)
            (`self.ExternalActivate` (`self.ApplyConditions`))))))))

(fn `AllActorsActive`
  (returns (OutputPin :type Boolean)))

(fn `Deactivate This`
  (params (Instigator :type "/Game/Lasers/Blueprints/BuildingBlocks/BPAC_Handler Object Reference"))
  (if (`self.InvertControl`)
    (set `self.IsCompActivated` false)
    (`self.ExternalDeactivate` (`self.ApplyConditions`))
    (else
      (`BlueprintMapLibrary.Map_Add` (`self.NecessaryActors`) (`local.Instigator`))
      (`self.ExternalDeactivate` (`self.ApplyConditions`)))))

(fn `Update This`
  (params (Alpha :type "Float (double-precision)"))
  (`self.ExternalUpdate` Alpha))