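; BPA_Book is a clickable 3D book that serves as a button in the game's menu.
; On BeginPlay it adds a WBP_HoverButton widget labeled "Play" to the viewport.
; Cursor-over events on its static mesh toggle a green highlight overlay material and show or hide that label.
; Clicking feeds a 180 yaw input to the player controller and opens WBP_Option with IsGameLaunched false.
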(event `self.ReceiveBeginPlay`
  (bind _returnvalue (`|CreateWidget` "/Game/Blueprint/UI/WBP_HoverButton.WBP_HoverButton_C" null "Play"))
  (bind _output_get (set `self.TxtWidget` _returnvalue))
  (`UserWidget.AddToViewport` _returnvalue 0)
  (`UserWidget.AddToViewport` _output_get 0))

(event `self.StaticMesh.OnBeginCursorOver`
  (params (TouchedComponent :type "PrimitiveComponent Object Reference"))
  (`MeshComponent.SetOverlayMaterial` (`self.StaticMesh`) "/Game/Material/MI_HighlightGreen.MI_HighlightGreen")
  (`/Game/Blueprint/UI/WBP_HoverButton.unhide text` (`self.TxtWidget`) "NewEnumerator1"))

(event `self.StaticMesh.OnEndCursorOver`
  (params (TouchedComponent :type "PrimitiveComponent Object Reference"))
  (`MeshComponent.SetOverlayMaterial` (`self.StaticMesh`) null)
  (`/Game/Blueprint/UI/WBP_HoverButton.hide text` (`self.TxtWidget`) "NewEnumerator1"))

(event `self.StaticMesh.OnClicked`
  (params (TouchedComponent :type "PrimitiveComponent Object Reference") (ButtonPressed :type "Key Structure"))
  (`PlayerController.AddYawInput` (`GameplayStatics.GetPlayerController` 0) 180.0)
  (bind _returnvalue (`|CreateWidget` "/Game/Blueprint/UI/WBP_Option.WBP_Option_C"))
  (`UserWidget.AddToViewport` _returnvalue 0))

(fn `UserConstructionScript`)