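; BPA_CrystalBall is a clickable crystal ball actor that serves as the menu's Play button, opening the ML_MasterLevel level when clicked.
; On begin play it adds a "Play" hover-button widget to the viewport and hides two components, NSBasic9 and NSBasic1.
; Cursor-over events on the static mesh show or hide the widget's text and those two components together.
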(event `self.ReceiveBeginPlay`
  (bind _returnvalue (`|CreateWidget` "/Game/Blueprint/UI/WBP_HoverButton.WBP_HoverButton_C" null "Play"))
  (bind _output_get (set `self.TxtWidget` _returnvalue))
  (`UserWidget.AddToViewport` _returnvalue 0)
  (`UserWidget.AddToViewport` _output_get 0)
  (`SceneComponent.SetVisibility` (`self.NS_Basic_9`) false false)
  (`SceneComponent.SetVisibility` (`self.NS_Basic_1`) false false))

(event `self.StaticMesh.OnBeginCursorOver`
  (params (TouchedComponent :type "PrimitiveComponent Object Reference"))
  (`/Game/Blueprint/UI/WBP_HoverButton.unhide text` (`self.TxtWidget`) "NewEnumerator0")
  (`SceneComponent.SetVisibility` (`self.NS_Basic_9`) true false)
  (`SceneComponent.SetVisibility` (`self.NS_Basic_1`) true false))

(event `self.StaticMesh.OnEndCursorOver`
  (params (TouchedComponent :type "PrimitiveComponent Object Reference"))
  (`/Game/Blueprint/UI/WBP_HoverButton.hide text` (`self.TxtWidget`) "NewEnumerator0")
  (`SceneComponent.SetVisibility` (`self.NS_Basic_9`) false false)
  (`SceneComponent.SetVisibility` (`self.NS_Basic_1`) false false))

(event `self.StaticMesh.OnClicked`
  (params (TouchedComponent :type "PrimitiveComponent Object Reference") (ButtonPressed :type "Key Structure"))
  (`GameplayStatics.OpenLevelBySoftObjectPtr` "/Game/Levels/ML_MasterLevel.ML_MasterLevel"))

(fn `UserConstructionScript`)