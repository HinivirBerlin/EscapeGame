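; BPA_Skull is a clickable skull actor for the menu that reveals effects on hover and quits the game on click.
; On BeginPlay it hides its NSBasic10 and Eyes components and adds a WBP_HoverButton widget to the viewport.
; Cursor events on the Cube component toggle both components and show or hide the widget's text.
; The widget is labelled "Play", although the click calls QuitGame.
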(event `self.ReceiveBeginPlay`
  (bind _returnvalue (`|CreateWidget` "/Game/Blueprint/UI/WBP_HoverButton.WBP_HoverButton_C" null "Play"))
  (bind _output_get (set `self.TxtWidget` _returnvalue))
  (`UserWidget.AddToViewport` _returnvalue 0)
  (`UserWidget.AddToViewport` _output_get 0)
  (`SceneComponent.SetVisibility` (`self.NS_Basic_10`) false false)
  (`SceneComponent.SetVisibility` (`self.eyes`) false false))

(event `self.Cube.OnBeginCursorOver`
  (params (TouchedComponent :type "PrimitiveComponent Object Reference"))
  (`/Game/Blueprint/UI/WBP_HoverButton.unhide text` (`self.TxtWidget`) "NewEnumerator2")
  (`SceneComponent.SetVisibility` (`self.NS_Basic_10`) true false)
  (`SceneComponent.SetVisibility` (`self.eyes`) true false))

(event `self.Cube.OnEndCursorOver`
  (params (TouchedComponent :type "PrimitiveComponent Object Reference"))
  (`/Game/Blueprint/UI/WBP_HoverButton.hide text` (`self.TxtWidget`) "NewEnumerator2")
  (`SceneComponent.SetVisibility` (`self.NS_Basic_10`) false false)
  (`SceneComponent.SetVisibility` (`self.eyes`) false false))

(event `self.Cube.OnClicked`
  (params (TouchedComponent :type "PrimitiveComponent Object Reference") (ButtonPressed :type "Key Structure"))
  (`KismetSystemLibrary.QuitGame` null "Quit"))

(fn `UserConstructionScript`)