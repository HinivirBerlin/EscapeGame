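; BPA_Paper is an interactable paper note that shows the player written story text in a UI widget.
; On BeginPlay, EnumText selects one of three hardcoded texts, the last being only a placeholder word.
; Interact hides the player HUD, switches to UI-only input with a visible cursor, and opens WBP_Paper with that text.
; Box overlaps toggle a green highlight overlay material on the paper.
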(event `self.ReceiveBeginPlay`
  (switch `/Game/Blueprint/Paper/E_PaperText` (`self.EnumText`)
    (:`NewEnumerator0`
      (set `self.TextToDisplay` "Where I am ? \nWhat is this place ? \nWhy this room has no ceiling ? \n \nDid I get kidnap during my investigation ? \n \nNo, I need to check where I am exactly and then find those who bring me here. \n \nBut still, what's happening ? \n \nSome kind of door prevents me from leaving the room \n \nI should probably see what I can find useful in this room. \n \nI will keep updating my progression, maybe someone will find those paper."))
    (:`NewEnumerator1`
      (set `self.TextToDisplay` "I'm still confused about the situation. \n \nHow did I end up here? \n \nI found notes left by people who were brought here too. Don't any of them know why? \n"))
    (:`NewEnumerator2`
      (set `self.TextToDisplay` "World"))))

(event `/Game/Blueprint/BPI_Interact.Interact`
  (params (Interactor :type "Character Object Reference"))
  (bind _returnvalue (`GameplayStatics.GetPlayerController` 0))
  (bind _asbp_player (cast `/Game/Blueprint/Player/BP_Player` (`GameplayStatics.GetPlayerPawn` 0)))
  (`Widget.SetVisibility` (`/Game/Blueprint/Player/BP_Player.Hud` _asbp_player) "Hidden")
  (`WidgetBlueprintLibrary.SetInputMode_UIOnlyEx` _returnvalue null)
  (set `PlayerController.bShowMouseCursor` true _returnvalue)
  (bind _returnvalue_2 (`|CreateWidget` "/Game/Blueprint/Paper/WBP_Paper.WBP_Paper_C" null (`self.TextToDisplay`)))
  (`UserWidget.AddToViewport` _returnvalue_2 0))

(event `self.Box.OnComponentBeginOverlap`
  (params (OverlappedComponent :type "PrimitiveComponent Object Reference") (OtherActor :type "Actor Object Reference") (OtherComp :type "PrimitiveComponent Object Reference") (OtherBodyIndex :type Integer) (bFromSweep :type Boolean) (SweepResult :type "HitResult Structure (by ref)"))
  (`MeshComponent.SetOverlayMaterial` (`self.Paper`) "/Game/Material/MI_HighlightGreen.MI_HighlightGreen"))

(event `self.Box.OnComponentEndOverlap`
  (params (OverlappedComponent :type "PrimitiveComponent Object Reference") (OtherActor :type "Actor Object Reference") (OtherComp :type "PrimitiveComponent Object Reference") (OtherBodyIndex :type Integer))
  (`MeshComponent.SetOverlayMaterial` (`self.Paper`) null))

(fn `UserConstructionScript`)